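; BP_Pawn is the player's camera pawn, providing pan, spring-arm zoom and stepped rotation.
; When a BP_PC controller takes over, it adds the default Enhanced Input mapping context.
; Input only updates desired location, rotation and clamped zoom, with movement relative to the pawn's facing and rotation in 45-degree steps.
; Tick interpolates the actor transform and arm length toward those targets for smooth motion.
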(event Input|EnhancedActionEvents|EnhancedInputActionIA_Zoom
  (params (ActionValue :type Float%20%28double-precision%29) (ElapsedSeconds :type Float%20%28double-precision%29) (TriggeredSeconds :type Float%20%28double-precision%29) (InputAction :type Input%20Action%20Object%20Reference :default "/Game/Blueprints/Core/Input/Action/IA_Zoom.IA_Zoom"))
  ;[0.15 0.15 0.15 0.5] IA_Zoom
  (:Triggered
    (Variables|Default|SetZoom_Desired (Math|Float|Clamp(Float) (+ (* ActionValue 1e+02) (Variables|Default|GetZoom_Desired)) 1e+02 5e+03))))

(event Input|EnhancedActionEvents|EnhancedInputActionIA_Move
  (params (ActionValue :type Vector%202D%20Structure) (ElapsedSeconds :type Float%20%28double-precision%29) (TriggeredSeconds :type Float%20%28double-precision%29) (InputAction :type Input%20Action%20Object%20Reference :default "/Game/Blueprints/Core/Input/Action/IA_Move.IA_Move"))
  ;[0.15 0.15 0.15 0.5] Move
  ;;[0.15 0.15 0.15 0.5] Left and Right
  (:Triggered
    (Variables|Default|SetLocation_Desired (+ (Variables|Default|GetLocation_Desired) (* (* (.X (Math|Vector2D|BreakVector2D ActionValue)) 4e+01) (Transformation|GetActorRightVector))))))

(event Input|EnhancedActionEvents|EnhancedInputActionIA_Move
  (params (ActionValue :type Vector%202D%20Structure) (ElapsedSeconds :type Float%20%28double-precision%29) (TriggeredSeconds :type Float%20%28double-precision%29) (InputAction :type Input%20Action%20Object%20Reference :default "/Game/Blueprints/Core/Input/Action/IA_Move.IA_Move"))
  ;[0.15 0.15 0.15 0.5] Move
  ;;[0.15 0.15 0.15 0.5] Up and Down
  (:Triggered
    (Variables|Default|SetLocation_Desired (+ (Variables|Default|GetLocation_Desired) (* (* (.Y (Math|Vector2D|BreakVector2D ActionValue)) 4e+01) (Transformation|GetActorForwardVector))))))

(event Input|EnhancedActionEvents|EnhancedInputActionIA_RotationLeft
  (params (ActionValue :type Boolean) (ElapsedSeconds :type Float%20%28double-precision%29) (TriggeredSeconds :type Float%20%28double-precision%29) (InputAction :type Input%20Action%20Object%20Reference :default "/Game/Blueprints/Core/Input/Action/IA_RotationLeft.IA_RotationLeft"))
  ;[0.15 0.15 0.15 0.5] Rotation Right and Left
  (:Started
    (Variables|Default|SetRotation_Desired (Math|Rotator|CombineRotators (Variables|Default|GetRotation_Desired) "0.000000,45.000000,0.000000"))))

(event Input|EnhancedActionEvents|EnhancedInputActionIA_RotationRight
  (params (ActionValue :type Boolean) (ElapsedSeconds :type Float%20%28double-precision%29) (TriggeredSeconds :type Float%20%28double-precision%29) (InputAction :type Input%20Action%20Object%20Reference :default "/Game/Blueprints/Core/Input/Action/IA_RotationRight.IA_RotationRight"))
  ;[0.15 0.15 0.15 0.5] Rotation Right and Left
  (:Started
    (Variables|Default|SetRotation_Desired (Math|Rotator|CombineRotators (Variables|Default|GetRotation_Desired) "0.000000,-45.000000,0.000000"))))

(event EventControllerChanged
  (params (OldController :type Controller%20Object%20Reference) (NewController :type Controller%20Object%20Reference))
  ;[0.15 0.15 0.15 0.5] EnhancedInput
  (bind _asbp_pc (Utilities|Casting|CastToBP_PC NewController))
  (Utilities|IsValid (PlayerController|LocalPlayerSubsystems|GetEnhancedInputLocalPlayerSubsystem _asbp_pc)
    (:Is%20Valid
      (Input|AddMappingContext (PlayerController|LocalPlayerSubsystems|GetEnhancedInputLocalPlayerSubsystem _asbp_pc) "/Game/Blueprints/Core/Input/IMC_Default.IMC_Default" 0 "(bIgnoreAllPressedKeysUntilRelease=True,bForceImmediately=False,bNotifyUserSettings=False)"))))

(event EventTick
  (params (DeltaSeconds :type Float%20%28single-precision%29))
  ;[0.15 0.15 0.15 0.5] Event Tick
  (Variables|/Script/Engine.SpringArmComponent|SetTargetArmLength (Variables|Default|GetSpringArm) (Math|Interpolation|FInterpTo (Variables|/Script/Engine.SpringArmComponent|GetTargetArmLength (Variables|Default|GetSpringArm)) (Variables|Default|GetZoom_Desired) DeltaSeconds 2.0))
  (Transformation|SetActorLocation (Math|Interpolation|VInterpTo (Transformation|GetActorLocation) (Variables|Default|GetLocation_Desired) DeltaSeconds 2.0) false false)
  (Transformation|SetActorRotation (Math|Interpolation|RInterpTo (Transformation|GetActorRotation) (Variables|Default|GetRotation_Desired) DeltaSeconds 5.0)))

(event EventBeginPlay
  ;[0.15 0.15 0.15 0.5] Event Begin Play
  (Variables|Default|SetLocation_Desired (Transformation|GetActorLocation))
  (Variables|Default|SetZoom_Desired (Variables|/Script/Engine.SpringArmComponent|GetTargetArmLength (Variables|Default|GetSpringArm)))
  (Variables|Default|SetRotation_Desired (Transformation|GetActorRotation)))

(fn ConstructionScript)